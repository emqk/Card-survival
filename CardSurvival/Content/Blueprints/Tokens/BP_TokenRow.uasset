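; BP_TokenRow is a token row Blueprint whose BeginPlay runs a hard-coded test sequence of adding and removing tokens.
; One-second delays space calls to AddToken and RemoveToken on two test token data assets, including one more removal of the first token than was added.
; The add and remove logic is not defined in this Blueprint, and its construction script is empty.
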(event `self.ReceiveBeginPlay`
  (`self.AddToken` "/Game/Data/Tokens/DA_TestToken.DA_TestToken")
  (`KismetSystemLibrary.Delay` 1.0)
  (`self.AddToken` "/Game/Data/Tokens/DA_TestToken.DA_TestToken")
  (`KismetSystemLibrary.Delay` 1.0)
  (`self.AddToken` "/Game/Data/Tokens/DA_TestToken2.DA_TestToken2")
  (`KismetSystemLibrary.Delay` 1.0)
  (`self.AddToken` "/Game/Data/Tokens/DA_TestToken2.DA_TestToken2")
  (`KismetSystemLibrary.Delay` 1.0)
  (`self.AddToken` "/Game/Data/Tokens/DA_TestToken2.DA_TestToken2")
  (`KismetSystemLibrary.Delay` 1.0)
  (`self.RemoveToken` "/Game/Data/Tokens/DA_TestToken.DA_TestToken")
  (`KismetSystemLibrary.Delay` 1.0)
  (`self.RemoveToken` "/Game/Data/Tokens/DA_TestToken.DA_TestToken")
  (`KismetSystemLibrary.Delay` 1.0)
  (`self.RemoveToken` "/Game/Data/Tokens/DA_TestToken.DA_TestToken")
  (`KismetSystemLibrary.Delay` 1.0)
  (`self.AddToken` "/Game/Data/Tokens/DA_TestToken.DA_TestToken"))

(fn `UserConstructionScript`)