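; BP_InteractionAim is an interaction aim visualizer that draws a curved spline mesh from a Start actor to an End position.
; RefreshMesh builds the curve from three points: start, offset midpoint and end.
; RefreshSplineMesh clears the previous visualization via HideVisualization, then creates spline mesh components between points using spline tangents.
; RefreshMesh also computes a launch velocity and predicted projectile path, but the prediction result is unused.
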(event `self.RefreshMesh`
  (bind _returnvalue (`self.K2_GetActorLocation` (`self.Start`)))
  (bind _outlaunchvelocity (`GameplayStatics.SuggestProjectileVelocity_CustomArc` (`self.K2_GetActorLocation` (`self.Start`)) (`self.End`)))
  (`GameplayStatics.Blueprint_PredictProjectilePath_ByObjectType` :`StartPos` (`self.K2_GetActorLocation` (`self.Start`)) :`LaunchVelocity` _outlaunchvelocity :`ProjectileRadius` 1.0 :`ObjectTypes` (`|MakeArray` "ObjectTypeQuery1" :!type "EObjectTypeQuery Enum") :`SimFrequency` 10.0)
  (`self.RefreshSplineMesh` (`|MakeArray` _returnvalue (+ (/ (+ _returnvalue (`self.End`)) 2.0) (`self.MidPointOffset`)) (`self.End`))))

(fn `HideVisualization`
  (for _array_element (`self.SplineMeshes`)
    (`ActorComponent.K2_DestroyComponent` _array_element))
  (`KismetArrayLibrary.Array_Clear` (`self.SplineMeshes`))
  (`SplineComponent.ClearSplinePoints` (`self.Spline`) true))

(fn `RefreshSplineMesh`
  (params (Points :type "Array of Vector Structure"))
  (locals (PointsLocal :type "Array of Vector Structure"))
  (`self.HideVisualization`)
  (bind _output_get (set `local.PointsLocal` Points))
  (for _array_element _output_get
    (`SplineComponent.AddSplinePoint` (`self.Spline`) _array_element "World" true))
  (for _index (range (+ (- (`SplineComponent.GetNumberOfSplinePoints` (`self.Spline`)) 2) 1))
    (bind _returnvalue (`AddComponent|NODE_AddSplineMeshComponent-0` :`bManualAttachment` true))
    (`SplineMeshComponent.SetStartScale` _returnvalue (`self.SplineScale`) false)
    (`SplineMeshComponent.SetEndScale` _returnvalue (`self.SplineScale`) false)
    (`KismetArrayLibrary.Array_Add` (`self.SplineMeshes`) _returnvalue)
    (bind _returnvalue_2 (+ _index 1))
    (`SplineMeshComponent.SetStartAndEnd` _returnvalue (`|GetArrayItem` (`local.PointsLocal`) _index) (`SplineComponent.GetTangentAtSplinePoint` (`self.Spline`) _index "World") (`|GetArrayItem` (`local.PointsLocal`) _returnvalue_2) (`SplineComponent.GetTangentAtSplinePoint` (`self.Spline`) _returnvalue_2 "World") true)))

(fn `UserConstructionScript`)