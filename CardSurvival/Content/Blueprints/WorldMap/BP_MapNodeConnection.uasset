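; BP_MapNodeConnection is a world map actor that draws a visual link between two map nodes, From and To.
; Its Connectto event clears previous meshes, then creates and attaches a spline mesh component using the configured Mesh, with its start and end set to the two nodes' locations.
; Created components are tracked in MeshComponents so ClearData can destroy them before each rebuild.
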(event `self.ConnectTo`
  (`self.ClearData`)
  (bind _returnvalue (`AddComponent|NODE_AddSplineMeshComponent-2`))
  (`KismetArrayLibrary.Array_Add` (`self.MeshComponents`) _returnvalue)
  (`StaticMeshComponent.SetStaticMesh` _returnvalue (`self.Mesh`))
  (`SceneComponent.K2_AttachToComponent` _returnvalue null "None" "KeepWorld" "KeepWorld" "KeepWorld" true)
  (`SplineMeshComponent.SetStartAndEnd` _returnvalue (`self.K2_GetActorLocation` (`self.From`)) (0.0 0.0 0.0) (`self.K2_GetActorLocation` (`self.To`)) (0.0 0.0 0.0) true))

(fn `ClearData`
  (for _array_element (`self.MeshComponents`)
    (`ActorComponent.K2_DestroyComponent` _array_element))
  (`KismetArrayLibrary.Array_Clear` (`self.MeshComponents`)))

(fn `UserConstructionScript`)