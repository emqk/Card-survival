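; BP_Card is a card Blueprint that shows its card info through the player's board pawn while selected.
; It overrides StartSelect and EndSelect, calling the parent version first, then telling the board pawn from the player subsystem to activate the info with this card's data or deactivate it.
; StartSelect returns true and EndSelect returns false, and the event graph holds no logic.
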(event `self.ReceiveBeginPlay`)

(fn `EndSelect`
  (params (Interactor :type "Actor Object Reference"))
  (returns (ReturnValue :type Boolean))
  (`parent.EndSelect` Interactor)
  (`PlayerBoardPawn.SetCardInfoActive` (`PlayerSubsystem.GetPlayerBoardPawn` (subsystem `PlayerSubsystem`)) null false)
  (return false))

(fn `StartSelect`
  (params (Interactor :type "Actor Object Reference"))
  (returns (ReturnValue :type Boolean))
  (`parent.StartSelect` Interactor)
  (`PlayerBoardPawn.SetCardInfoActive` (`PlayerSubsystem.GetPlayerBoardPawn` (subsystem `PlayerSubsystem`)) (`self.GetCardData`) true)
  (return true))

(fn `UserConstructionScript`)