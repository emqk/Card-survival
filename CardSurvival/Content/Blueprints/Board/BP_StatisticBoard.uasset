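; BP_StatisticBoard is a board actor that displays the player's gold, health, energy and sanity.
; On BeginPlay it binds refresh events to each attribute's change delegate from PlayerInventorySubsystem, then runs an initial refresh.
; Health, energy and sanity share RefreshBarBase, which scales a bar mesh's world Y by the normalized amount times a maximum scale and updates its WBP_StatisticAmount text.
; Gold updates only its text widget.
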(event `self.ReceiveBeginPlay`
  (bind _returnvalue (subsystem `PlayerInventorySubsystem`))
  ;[1 0.07057 0.5787] Bind events
  (add `Statistic.OnAttributeChange` (`PlayerInventorySubsystem.GetGold` (subsystem `PlayerInventorySubsystem`)) (`|CreateDelegate` :!event `RefreshGold`))
  (add `Statistic.OnAttributeChange` (`PlayerInventorySubsystem.GetHealth` (subsystem `PlayerInventorySubsystem`)) (`|CreateDelegate` :!event `RefreshHealthBar`))
  (add `Statistic.OnAttributeChange` (`PlayerInventorySubsystem.GetEnergy` (subsystem `PlayerInventorySubsystem`)) (`|CreateDelegate` :!event `RefreshEnergyBar`))
  (add `Statistic.OnAttributeChange` (`PlayerInventorySubsystem.GetSanity` (subsystem `PlayerInventorySubsystem`)) (`|CreateDelegate` :!event `RefreshSanityBar`))
  ;[0.2853 0 1] Initial refresh
  (`self.RefreshGold` (`PlayerInventorySubsystem.GetGold` _returnvalue))
  (`self.RefreshHealthBar` (`PlayerInventorySubsystem.GetHealth` _returnvalue))
  (`self.RefreshEnergyBar` (`PlayerInventorySubsystem.GetEnergy` _returnvalue))
  (`self.RefreshSanityBar` (`PlayerInventorySubsystem.GetSanity` _returnvalue)))

(event `RefreshGold`
  (params (ModifiedStatistic :type "Statistic Object Reference"))
  (`/Game/Blueprints/Board/WBP_StatisticAmount.RefreshText` (cast `/Game/Blueprints/Board/WBP_StatisticAmount` (`WidgetComponent.GetWidget` (`self.GoldText`)) :!pure true) (`Statistic.GetAmount` ModifiedStatistic)))

(event `RefreshHealthBar`
  (params (ModifiedStatistic :type "Statistic Object Reference"))
  (`self.RefreshBarBase` ModifiedStatistic (`self.HealthBarComponent`) (cast `/Game/Blueprints/Board/WBP_StatisticAmount` (`WidgetComponent.GetWidget` (`self.HealthText`)) :!pure true)))

(event `RefreshEnergyBar`
  (params (ModifiedStatistic :type "Statistic Object Reference"))
  (`self.RefreshBarBase` ModifiedStatistic (`self.EnergyBarComponent`) (cast `/Game/Blueprints/Board/WBP_StatisticAmount` (`WidgetComponent.GetWidget` (`self.EnergyText`)) :!pure true)))

(event `RefreshSanityBar`
  (params (ModifiedStatistic :type "Statistic Object Reference"))
  (`self.RefreshBarBase` ModifiedStatistic (`self.SanityBarComponent`) (cast `/Game/Blueprints/Board/WBP_StatisticAmount` (`WidgetComponent.GetWidget` (`self.SanityText`)) :!pure true)))

(event `RefreshBarBase`
  (params (ModifiedStatistic :type "Statistic Object Reference") (BarMesh :type "StaticMeshComponent Object Reference") (WidgetText :type "/Game/Blueprints/Board/WBP_StatisticAmount Object Reference"))
  (bind (_returnvalue_x _returnvalue_y _returnvalue_z) (`KismetMathLibrary.BreakVector` (`SceneComponent.K2_GetComponentScale` BarMesh)))
  (`SceneComponent.SetWorldScale3D` BarMesh (`KismetMathLibrary.MakeVector` _returnvalue_x (* (`self.GetMaxBarScale`) (`Statistic.GetAmountNormalized` ModifiedStatistic)) _returnvalue_z))
  (`/Game/Blueprints/Board/WBP_StatisticAmount.RefreshText` WidgetText (`Statistic.GetAmount` ModifiedStatistic)))

(fn `UserConstructionScript`)